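; Base backpack actor the first-person character picks up by overlap, attaching it to a spine socket hidden from its owner.
; On BeginPlay it spawns pocket objects from PocketDetails and builds each a centered grid of 3D tile widgets, filling inventory with -1.
; Toggle events flip tile and owner visibility.
; PutItemInBackpack overlays a size-scaled item widget on hardcoded pocket index 2, without updating inventory.
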(event OnComponentBeginOverlap(Sphere)
  (params (OverlappedComponent :type Primitive%20Component%20Object%20Reference) (OtherActor :type Actor%20Object%20Reference) (OtherComp :type Primitive%20Component%20Object%20Reference) (OtherBodyIndex :type Integer) (bFromSweep :type Boolean) (SweepResult :type Hit%20Result%20Structure%20%28by%20ref%29))
  (bind _asbp_first_person_character (Utilities|Casting|CastToBP_FirstPersonCharacter OtherActor))
  (bind _output_get (Variables|Default|SetPersonReference _asbp_first_person_character))
  (Actor|SetOwner _output_get)
  (bind _output_get_2 (Variables|/Game/FirstPerson/Blueprints/BP_FirstPersonCharacter.BP_FirstPersonCharacter_C|SetBackpack _output_get self))
  (Collision|SetActorEnableCollision _output_get_2 false)
  (CallFunction|AttachtoSpine (Variables|/Script/Engine.Character|GetMesh _output_get)))

(event Custom|ToggleBackpackVisibility
  (bind _isa (Utilities|FlowControl|FlipFlop)
    (:A
      _)
    (:B
      _))
  (CallFunction|ToggleWidgetVisibility)
  (Class|PrimitiveComponent|SetOwnerNoSee (Variables|Default|GetBackpackComponent) (not _isa)))

(event Custom|ToggleWidgetVisibility
  (bind _isa (Utilities|FlowControl|FlipFlop)
    (:A
      _)
    (:B
      _))
  (for _array_element (Variables|Default|GetPockets)
    (for _array_element_2 (Variables|/Game/Backpacks/BP_PocketVariable.BP_PocketVariable_C|GetBoxes _array_element)
      (Rendering|SetVisibility _array_element_2 (not _isa) false))))

(event Custom|AttachToActor
  (params (NewParam :type Actor%20Object%20Reference) (RelativeLocation :type Vector))
  (Transformation|AttachActorToActor NewParam "None" "SnapToTarget" "SnapToTarget" "SnapToTarget" true)
  (Class|PrimitiveComponent|SetOwnerNoSee (Variables|Default|GetBackpackComponent) false)
  (Transformation|SetActorRelativeTransform (Math|Transform|MakeTransform RelativeLocation) false false))

(event Custom|AttachToSpine
  (params (NewParam :type Scene%20Component%20Object%20Reference))
  (Transformation|AttachComponentToComponent NewParam "BackpackSocket" "SnapToTarget" "SnapToTarget" "SnapToTarget" true)
  (Class|PrimitiveComponent|SetOwnerNoSee (Variables|Default|GetBackpackComponent) true))

(event Custom|PutItemInBackpack
  (params (Item :type BP%20Item%20Master%20Object%20Reference))
  (bind _itemproperties (Variables|/Game/Items/BP_ItemMaster.BP_ItemMaster_C|GetItemProperties Item))
  (bind _sizeinbackpack (Utilities|Struct|BreakS_ItemProperties _itemproperties))
  (bind (_x _y) (Math|Vector2D|BreakVector2D _sizeinbackpack))
  (bind _returnvalue (Math|Vector|MakeVector _x _y _x))
  (bind _returnvalue_2 (UserInterface|CreateWidget "/Game/Items/W_Item.W_Item_C"))
  (Default|SetImage _returnvalue_2 (Variables|/Game/Items/BP_ItemMaster.BP_ItemMaster_C|GetImage Item))
  (Development|PrintString "Hello")
  (bind _returnvalue_3 (AddComponent|AddWidgetComponent false (Math|Transform|MakeTransform (Utilities|NewMacro _returnvalue 0 0 2) "90.000000,0.000000,180.000000" (* "0.001000,0.001000,0.001000" (* (Variables|Default|GetBoxSize) _returnvalue "2.000000,2.000000,2.000000")))))
  (UserInterface|SetWidget _returnvalue_3 _returnvalue_2)
  (Rendering|SetTranslucentSortPriority _returnvalue_3 1))

(event EventBeginPlay
  (CallFunction|InitializePockets)
  (CallFunction|CreateTiles)
  (CallFunction|ToggleWidgetVisibility)
  (bind _asprimitive_component (Utilities|Casting|CastToPrimitiveComponent (Components|GetChildComponent (Variables|Default|GetEmptyParent) 0)))
  (Variables|Default|SetBackpackComponent _asprimitive_component))

(fn ConstructionScript)

(fn InitializePockets
  (for _array_element (Variables|Default|GetPocketDetails)
    (bind _returnvalue (Game|SpawnActorfromClass "/Game/Backpacks/BP_PocketVariable.BP_PocketVariable_C" (Math|Transform|MakeTransform "0, 0, 0") "Undefined" "MultiplyWithRoot" 0 0))
    (Variables|/Game/Backpacks/BP_PocketVariable.BP_PocketVariable_C|SetSize _returnvalue (.Size (Utilities|Struct|BreakS_Pocket _array_element)))
    (Variables|/Game/Backpacks/BP_PocketVariable.BP_PocketVariable_C|SetLocation _returnvalue (.Location (Utilities|Struct|BreakS_Pocket _array_element)))
    (Utilities|Array|Add (Variables|Default|GetPockets) _returnvalue))
  (return))

(fn CreateTiles
  (bind _boxsize (Variables|Default|GetBoxSize))
  (bind (_x _y) (Math|Vector|BreakVector _boxsize))
  (for _array_element (Variables|Default|GetPockets)
    (for _index (range 0 (Math|Float|Truncate (- (Math|Float|Truncate (.X (Math|Vector|BreakVector (Variables|/Game/Backpacks/BP_PocketVariable.BP_PocketVariable_C|GetSize _array_element)))) 1)))
      (for _index_2 (range 0 (Math|Float|Truncate (- (Math|Float|Truncate (.Y (Math|Vector|BreakVector (Variables|/Game/Backpacks/BP_PocketVariable.BP_PocketVariable_C|GetSize _array_element)))) 1)))
        (Utilities|Array|Add (Variables|/Game/Backpacks/BP_PocketVariable.BP_PocketVariable_C|GetInventory _array_element) -1)
        (bind _returnvalue (UserInterface|CreateWidget "/Game/Backpacks/W_Tile.W_Tile_C"))
        (bind _returnvalue_2 (AddComponent|AddWidgetComponent false (Math|Transform|MakeTransform (+ (* (+ (Math|Vector|MakeVector (* _index _x) (* _index_2 _y) 25.0) (* (Math|Vector|MakeVector (* _x (- (Math|Float|Truncate (.X (Math|Vector|BreakVector (Variables|/Game/Backpacks/BP_PocketVariable.BP_PocketVariable_C|GetSize _array_element)))) 1)) (* _y (- (Math|Float|Truncate (.Y (Math|Vector|BreakVector (Variables|/Game/Backpacks/BP_PocketVariable.BP_PocketVariable_C|GetSize _array_element)))) 1)) 25.0) "-0.500000,-0.500000,-0.500000") (Variables|/Game/Backpacks/BP_PocketVariable.BP_PocketVariable_C|GetLocation _array_element)) "1.000000,1.000000,0.000000") (Math|Vector|MakeVector 0.0 0.0 (Variables|Default|GetHeightOfTiles))) "90.000000,0.000000,180.000000" (* "0.001000,0.001000,0.001000" (* (Variables|Default|GetBoxSize) "2.000000,2.000000,2.000000")))))
        (UserInterface|SetWidget _returnvalue_2 _returnvalue)
        (Rendering|Material|SetMaterial _returnvalue_2 0 "/Engine/EngineMaterials/Widget3DPassThrough.Widget3DPassThrough")
        (Utilities|Array|Add (Variables|/Game/Backpacks/BP_PocketVariable.BP_PocketVariable_C|GetBoxes _array_element) _returnvalue_2)
        (Transformation|AttachComponentToComponent _returnvalue_2 (Variables|Default|GetDefaultSceneRoot) "None" "KeepRelative" "KeepRelative" "KeepRelative" true)))))