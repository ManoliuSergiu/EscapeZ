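; BP_Photobooth is an editor photobooth actor that renders portraits of static meshes through a SceneCapture2D.
; GeneratePortrait assigns the given mesh, rotates the directional light and spring arm to the given rotation, and restricts the capture to that mesh component.
; It sizes the ortho width from the mesh's bounding sphere and places the capture component from the bounds origin and X extent.
; A separate custom event triggers the scene capture.
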(event Custom|GeneratePortrait
  (params (SM :type Static%20Mesh%20Object%20Reference) (Rotation :type Rotator))
  (bind _returnvalue (StaticMesh|GetBounds SM))
  (Transformation|SetRelativeRotation (Variables|Default|GetDirectionalLight) Rotation false false)
  (Transformation|SetRelativeRotation (Variables|Default|GetSpringArm) Rotation false false)
  (Components|StaticMesh|SetStaticMesh (Variables|Default|GetStaticMesh) SM)
  (Variables|/Script/Engine.SceneCaptureComponent2D|SetOrthoWidth (Variables|Default|GetSceneCaptureComponent2D) (* (.sphereradius _returnvalue) 2.1))
  (Transformation|SetRelativeLocation (Variables|Default|GetSceneCaptureComponent2D) (+ (.origin _returnvalue) (Math|Vector|MakeVector (* (.x (.boxextent _returnvalue)) 3.0) 0.0 0.0)) false true)
  (Rendering|SceneCapture|ShowOnlyComponent (Variables|Default|GetSceneCaptureComponent2D) (Variables|Default|GetStaticMesh)))

(event Custom|CustomEvent
  (Rendering|SceneCapture|CaptureScene (Variables|Default|GetSceneCaptureComponent2D) :!class /Script/Engine.SceneCaptureComponent2D))

(fn ConstructionScript)