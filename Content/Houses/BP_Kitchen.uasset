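; Kitchen Blueprint that sets up its drawers and cupboards as interactive parts when play begins.
; It scans all child components and tags those with Drawer, Cupboard or vert in their names as Interactive.
; A switch on a key built from those name matches spawns a drawer, cupboard or V-variant cupboard helper actor, passing it the component.
; Tagged components and spawned helpers are kept in arrays.
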(event EventBeginPlay
  (bind _returnvalue (Math|Transform|MakeTransform "0, 0, 0"))
  (bind _output_get (Variables|Default|SetAllComponents (Components|GetChildrenComponents (Variables|Default|GetDefaultSceneRoot) true)))
  (for _array_element _output_get
    (if (Math|Boolean|ORBoolean (Utilities|String|Contains (Utilities|GetObjectName _array_element) "Drawer") (Utilities|String|Contains (Utilities|GetObjectName _array_element) "Cupboard") (Utilities|String|Contains (Utilities|GetObjectName _array_element) "vert"))
      (Variables|/Script/Engine.ActorComponent|SetComponentTags _array_element (Utilities|Array|MakeArray "Interactive"))
      (Utilities|Array|Add (Variables|Default|GetInteractiveComponents) _array_element)
      (switch string (Utilities|String|Append (Utilities|String|SelectString "Drawer" "" (Utilities|String|Contains (Utilities|GetObjectName _array_element) "Drawer")) (Utilities|String|SelectString "Cupboard" "" (Utilities|String|Contains (Utilities|GetObjectName _array_element) "Cupboard")) (Utilities|String|SelectString "V" "" (Utilities|String|Contains (Utilities|GetObjectName _array_element) "vert")))
        (:Drawer
          (bind _returnvalue_2 (Game|SpawnActorfromClass "/Game/WorldInteraction/DrawerComponent2.DrawerComponent2_C" _returnvalue "Undefined" "MultiplyWithRoot" 0 _array_element 0 0))
          (Utilities|Array|Add (Variables|Default|GetActor) _returnvalue_2))
        (:Cupboard
          (bind _returnvalue_3 (Game|SpawnActorfromClass "/Game/WorldInteraction/CupboardComponent2.CupboardComponent2_C" _returnvalue "Undefined" "MultiplyWithRoot" 0 _array_element 0 0))
          (Utilities|Array|Add (Variables|Default|GetActor) _returnvalue_3))
        (:CupboardV
          (bind _returnvalue_4 (Game|SpawnActorfromClass "/Game/WorldInteraction/CupboardVComponent2.CupboardVComponent2_C" _returnvalue "Undefined" "MultiplyWithRoot" 0 _array_element 0 0))
          (Utilities|Array|Add (Variables|Default|GetActor) _returnvalue_4))))))

(event Collision|EventActorBeginOverlap
  (params (OtherActor :type Actor%20Object%20Reference)))

(event EventTick
  (params (DeltaSeconds :type Float%20%28single-precision%29)))

(fn ConstructionScript)