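; BP_Sharp is a weapon item Blueprint for sharp weapons that defines how their damage is calculated.
; GetDamage adds a random bonus between zero and RandomDamage to BaseDamage, then multiplies the sum by Sharpness.
; The event graph holds only disabled placeholder BeginPlay and Tick events, so the damage formula is its only active logic.
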(event EventBeginPlay
  (|CallParentFunction) ; This node is disabled and will not be called.\nDrag off pins to build functionality.
)

(event EventTick
  (params (DeltaSeconds :type Float%20%28single-precision%29))
  (|CallParentFunction DeltaSeconds) ; This node is disabled and will not be called.\nDrag off pins to build functionality.
)

(fn GetDamage
  (return (* (+ (Variables|Default|GetBaseDamage) (Math|Random|RandomFloatinRange 0.0 (Variables|Default|GetRandomDamage))) (Variables|Default|GetSharpness))))