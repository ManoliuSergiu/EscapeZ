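; Item spawner that fills an inventory, supplied through GetInventory, with random items matching its category filters.
; On BeginPlay it collects child secondary-category components as filters, then after a short delay filters the GameState's item classes by main type and category.
; A macro compares subtypes per category, though Clothing, Gardening and Junk outputs are unwired, so never qualify items.
; It spawns random picks once per roll into the backpack, printing debug text throughout.
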(event Custom|GetInventory
  (params (In :type Interaction%20Component%202%20Object%20Reference))
  (Variables|Default|SetInteractiveComponent In))

(event Custom|SpawnItems
  (bind _spawnableitems (Variables|Default|GetSpawnableItems))
  (for _index (range 1 (Variables|Default|GetRolls))
    (bind _returnvalue (Game|SpawnActorfromClass (Utilities|Array|Get(acopy) _spawnableitems (Math|Random|RandomInteger (Utilities|Array|Length _spawnableitems))) (Math|Transform|MakeTransform "0, 0, 0") "Undefined" "MultiplyWithRoot" 0 0))
    (Default|PutIteminBackpack (Variables|Default|GetInteractiveComponent) _returnvalue)
    (Development|PrintString (Utilities|String|Append "Spawned a " (Utilities|GetDisplayName _returnvalue)) true true "(R=0.400448,G=1.000000,B=0.245600,A=1.000000)" 213.0)))

(event EventBeginPlay
  (for _array_element (Components|GetChildrenComponents false)
    (bind _asbp_secondary_category (Utilities|Casting|CastToBP_SecondaryCategory _array_element))
    (Utilities|Array|Add (Variables|Default|GetFilters) _asbp_secondary_category))
  (Utilities|FlowControl|Delay 0.2)
  (CallFunction|FilterItems)
  (Development|PrintString (Utilities|String|ToString(Integer) (Utilities|Array|Length (Variables|Default|GetSpawnableItems))))
  (CallFunction|SpawnItems))

(fn FilterItems
  (bind _asbp_gs_gamestate (Utilities|Casting|CastToBP_GS_Gamestate (Game|GetGameState)))
  (for (_array_element _array_index) (Variables|/Game/FirstPerson/Blueprints/BP_GS_Gamestate.BP_GS_Gamestate_C|GetItemClasses _asbp_gs_gamestate)
    (Development|PrintString (Utilities|GetClassDisplayName _array_element) true true "(R=1.000000,G=0.582738,B=0.572790,A=1.000000)" 312.0)
    (if (== (Variables|Default|GetMainCategories) (.ItemType (Utilities|GetClassDefaults _array_element)))
      (Utilities|Array|Add (Variables|Default|GetSpawnableItems) _array_element)
      (LocalVariables|SetNewLocalVar false)
      (bind _array_element_2 (Utilities|Array|ForEachLoopwithBreak (Variables|/Game/Items/Blueprints/BP_ItemMaster.BP_ItemMaster_C|GetCategories (Utilities|Array|Get(acopy) (Variables|/Game/FirstPerson/Blueprints/BP_GS_Gamestate.BP_GS_Gamestate_C|GetItems _asbp_gs_gamestate) _array_index)))
        (:LoopBody
          (Development|PrintString (Utilities|GetDisplayName _array_element_2) true true "(R=0.000000,G=0.012712,B=1.000000,A=123.000000)" 1232.0)
          (for _array_element_3 (Variables|Default|GetFilters)
            (if (Utilities|Enum|Equal(Enum) (Variables|/Game/Items/ItemCategories/BP_SecondaryCategory.BP_SecondaryCategory_C|GetCategory _array_element_2) (Variables|/Game/Items/ItemCategories/BP_SecondaryCategory.BP_SecondaryCategory_C|GetCategory _array_element_3))
              (Utilities|NewMacro _array_element_3 _array_element_2 (Variables|/Game/Items/ItemCategories/BP_SecondaryCategory.BP_SecondaryCategory_C|GetCategory _array_element_3)
                (:Weapons
                  _)
                (:Equipment
                  _)
                (:Food
                  _)
                (:Medical
                  _)
                (:ReadingMaterials
                  _)
                (:Materials
                  _))
              (LocalVariables|SetNewLocalVar true))))
        (:Completed
          (if (not (LocalVariables|GetNewLocalVar))
            (Utilities|Array|RemoveItem (Variables|Default|GetSpawnableItems) _array_element)))))))